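; Monitor is an actor that displays the current frame rate in the world through a TextRender component.
; Each Tick it computes one over delta seconds, sets that as the text and also prints it to screen.
; Leftover unwired nodes include a camera-facing rotation calculation and a test print.
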(event EventBeginPlay)

(event EventTick
  (params (DeltaSeconds :type Float%20%28single-precision%29))
  (bind _returnvalue (/ 1.0 DeltaSeconds))
  (bind _returnvalue_2 (Utilities|Text|ToText(Float) _returnvalue "HalfToEven"))
  (Rendering|Components|TextRender|SetText (Variables|Default|GetTextRender) _returnvalue_2)
  (Development|PrintString (Utilities|String|ToString(Text) _returnvalue_2)))

(fn ConstructionScript)