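; BP_PickupCube is a grabbable physics object that a VR pawn can pick up and drop.
; Pickup turns off mesh physics simulation and attaches the root to the supplied component, keeping its world transform.
; Drop restores physics and detaches the actor in place.
; Grab and LockorRelease are empty, and a gated FlipFlop that would send socket and transform data to the pawn is disconnected, so it never runs.
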(event EventPickup
  (params (AttachTo :type Scene%20Component%20Object%20Reference) (RightHand? :type Boolean))
  ;[1 1 1] turn on collision generates hit events an no collision for this
  (Physics|SetSimulatePhysics (Variables|Debug|GetStaticMeshComponent) false)
  (Transformation|AttachComponentToComponent (VehicleSound|GetRootComponent) AttachTo "None" "KeepWorld" "KeepWorld" "KeepWorld" false))

(event EventDrop
  ;[1 1 1] turn on collision generates hit events an no collision for this
  (Physics|SetSimulatePhysics (Variables|Debug|GetStaticMeshComponent) true)
  (Transformation|DetachFromActor "KeepWorld" "KeepWorld" "KeepWorld"))

(event EventGrab
  (params (Pawn :type Actor%20Object%20Reference))
  ;[0 0.3566 1] Grab
)

(event EventLockorRelease
  ;[0 0.3566 1] Grab
)

(fn ConstructionScript)