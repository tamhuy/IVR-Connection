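; Actor for a 3D image display with an attached menu widget for scaling, removing its border and closing it.
; On BeginPlay it binds the 3dImage widget's events to its own handlers.
; Close and scale go through VRPawnInteraction_P on player pawn 0, with scaling also applied locally in fixed increments.
; Border removal hides the Back component and all four menu buttons directly, leaving the pawn's RemoveBorder call unconnected.
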(event Custom|RemoveBorderMulticast
  (Rendering|SetVisibility (Variables|Default|GetBack) false false)
  (CallFunction|SetButtonVisibility))

(event Custom|Scale
  (params (ScaleUp? :type Boolean))
  (bind _returnvalue (Transformation|GetActorScale3D))
  (bind _returnvalue_2 (Transformation|GetActorScale3D))
  (bind _scaleincrement (Variables|Default|GetScaleIncrement))
  (bind _scaleincrement_2 (Variables|Default|GetScaleIncrement))
  (bind _returnvalue_3 (- _returnvalue_2 _scaleincrement_2))
  (bind _returnvalue_4 (+ _returnvalue _scaleincrement))
  (if ScaleUp?
    (CallFunction|SetScale _returnvalue_4)
    (bind _asvrpawn_interaction_p (Utilities|Casting|CastToVRPawnInteraction_P (Game|Player|GetPlayerPawn 0)))
    (Default|SetImageScale _asvrpawn_interaction_p self _returnvalue_4)
    (else
      (CallFunction|SetScale _returnvalue_3)
      (bind _asvrpawn_interaction_p_2 (Utilities|Casting|CastToVRPawnInteraction_P (Game|Player|GetPlayerPawn 0)))
      (Default|SetImageScale _asvrpawn_interaction_p_2 self _returnvalue_3))))

(event Custom|SetButtonVisibility
  (bind _as3d_image (Utilities|Casting|CastTo3dImage (UserInterface|GetUserWidgetObject (Variables|Default|GetMenu))))
  (Widget|SetVisibility (Variables|/Game/UI/AllLevels/3dImage.3dImage_C|GetScaleDown _as3d_image) "Hidden")
  (Widget|SetVisibility (Variables|/Game/UI/AllLevels/3dImage.3dImage_C|GetScaleUp _as3d_image) "Hidden")
  (Widget|SetVisibility (Variables|/Game/UI/AllLevels/3dImage.3dImage_C|GetRemoveBorderButton _as3d_image) "Hidden")
  (Widget|SetVisibility (Variables|/Game/UI/AllLevels/3dImage.3dImage_C|GetCloseImage _as3d_image) "Hidden"))

(event Custom|DestroyThis
  (bind _returnvalue (Game|Player|GetPlayerPawn 0))
  (Development|PrintString (Utilities|GetDisplayName _returnvalue) false)
  (bind _asvrpawn_interaction_p (Utilities|Casting|CastToVRPawnInteraction_P _returnvalue))
  (Default|DestroyImage _asvrpawn_interaction_p self))

(event Custom|RemoveBorderEvent
  (CallFunction|RemoveBorder))

(event Custom|RemoveBorder
  (CallFunction|RemoveBorderMulticast))

(event Custom|setScale
  (params (NewParam :type Vector))
  (Transformation|SetActorScale3D NewParam))

(event EventBeginPlay
  (bind _as3d_image (Utilities|Casting|CastTo3dImage (UserInterface|GetUserWidgetObject (Variables|Default|GetMenu))))
  (EventDispatchers|BindEventtoCloseImageEvent _as3d_image (delegate Custom|DestroyThis))
  (EventDispatchers|BindEventtoScaleEvent _as3d_image (delegate Custom|Scale))
  (EventDispatchers|BindEventtoRemoveBorder _as3d_image (delegate Custom|RemoveBorderEvent)))

(fn ConstructionScript
  (|CallParentFunction))