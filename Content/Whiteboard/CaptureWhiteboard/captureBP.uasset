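; Capture actor that saves a high-resolution image of the in-game whiteboard to the Dropbox path stored in the player's settings save.
; On BeginPlay it reads that path and, after a short delay, binds its capture event to the VR pawn's whiteboard capture trigger.
; Each capture renders the SceneCapture2D into a new render target and writes it under an unused filename, found by rescanning the folder with an incrementing numeric prefix.
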(event Custom|captureEvent
  (bind _capturecomponent2d (Variables|DecalActor|GetCaptureComponent2D))
  (Variables|/Script/Engine.SceneCaptureComponent2D|SetTextureTarget _capturecomponent2d (Class|BrowseFiles|CreateRenderTarget2DTexture 4096 2384))
  (Rendering|SceneCapture|CaptureScene _capturecomponent2d :!class /Script/Engine.SceneCaptureComponent2D)
  (bind _unusedpath (CallFunction|FindUnusedPath))
  (Development|PrintString _unusedpath)
  (bind _returnvalue (Class|BrowseFiles|ModifiedCaptureComponent2DSaveImage (Variables|DecalActor|GetCaptureComponent2D) _unusedpath))
  (Development|PrintString (Utilities|String|ToString(Boolean) _returnvalue) false))

(event EventBeginPlay
  (bind _returnvalue (SaveGame|LoadGamefromSlot "PlayerSettingsSave"))
  (bind _asplayer_save_game (Utilities|Casting|CastToPlayerSaveGame _returnvalue))
  (Variables|Default|SetSavePath (.dropboxpath (Variables|/Game/Gameplay/PlayerSaveGame.PlayerSaveGame_C|GetS_PlayerInfo _asplayer_save_game)))
  (Utilities|FlowControl|Delay 1.0)
  (bind _asvrpawn_interaction_p (Utilities|Casting|CastToVRPawnInteraction_P (Game|Player|GetPlayerPawn 0))
    (:then
      (EventDispatchers|BindEventtoCaptureWhiteboard _asvrpawn_interaction_p (delegate Custom|captureEvent)))
    (:CastFailed
      (Development|PrintString "in captureBP: pawn cast failed"))))

(fn ConstructionScript)

(fn FindUnusedPath
  (LocalVariables|SetNewFileName (Variables|Default|Getfilename))
  (bind _array_element (Utilities|Array|ForEachLoopwithBreak (.Files (Class|BrowseFiles|GetFilesandFolders (Variables|Default|GetSavePath))) :!label _label)
    (:LoopBody
      (bind _output_get (LocalVariables|SetEqualName? (Utilities|Enum|Equal(Enum) _array_element (LocalVariables|GetNewFileName))))
      (if _output_get
        (goto _label Break)))
    (:Completed
      (if _output_get
        (LocalVariables|SetNewFileName (Utilities|String|Append (Variables|Default|GetFilenameAppend) (Variables|Default|Getfilename)))
        (Variables|Default|SetFilenameAppend (Utilities|String|ToString(Integer) (+ (Math|Conversions|ToInteger(Byte) (Variables|Default|GetFilenameAppend)) 1)))
        (goto _label)
        (else
          (return (Utilities|String|Append (Utilities|String|Append (Variables|Default|GetSavePath) "\\") (LocalVariables|GetNewFileName))))))))